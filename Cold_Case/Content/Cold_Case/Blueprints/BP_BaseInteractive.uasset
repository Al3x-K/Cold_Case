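; BP_BaseInteractive is a base actor for objects the player can interact with.
; Its ProximityVolume shows the InteractWidget when a BP_Player begins overlapping and hides it when the overlap ends.
; The OnInteract event plays InteractionSound at the actor's location, and nothing in this Blueprint calls it.
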(event OnComponentBeginOverlap(ProximityVolume)
  (params (OverlappedComponent :type Primitive%20Component%20Object%20Reference) (OtherActor :type Actor%20Object%20Reference) (OtherComp :type Primitive%20Component%20Object%20Reference) (OtherBodyIndex :type Integer) (bFromSweep :type Boolean) (SweepResult :type Hit%20Result%20Structure%20%28by%20ref%29))
  (Utilities|Casting|CastToBP_Player OtherActor)
  (Rendering|SetVisibility (Variables|Default|GetInteractWidget) true false))

(event OnComponentEndOverlap(ProximityVolume)
  (params (OverlappedComponent :type Primitive%20Component%20Object%20Reference) (OtherActor :type Actor%20Object%20Reference) (OtherComp :type Primitive%20Component%20Object%20Reference) (OtherBodyIndex :type Integer))
  (Utilities|Casting|CastToBP_Player OtherActor)
  (Rendering|SetVisibility (Variables|Default|GetInteractWidget) false false))

(event EventOnInteract
  (params (Interactor :type Actor%20Object%20Reference))
  (Audio|PlaySoundatLocation (Variables|Default|GetInteractionSound) (Transformation|GetActorLocation) "0, 0, 0" 1.0 1.0 0.0 0 0 0 0))

(fn ConstructionScript)