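; BP_Door is an interactive door that serves as the game's exit, opening only when the player's inventory contains "Keys".
; On interaction it checks the BP_Player inventory, plays an unlock sound at the door and runs the DoorSequence level sequence.
; When the sequence finishes, the camera fades out and the game quits after a short delay.
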(event Custom|OnFinished_Event_0
  (CameraFades|StartCameraFade :self (Game|GetPlayerCameraManager 0) :ToAlpha 1.0 :Duration 1.0)
  (Utilities|FlowControl|Delay 1.0)
  (Game|QuitGame (Game|GetPlayerController 0) "Quit" false))

(event EventExecuteInteraction
  (bind _asbp_player (Utilities|Casting|CastToBP_Player (Game|GetPlayerCharacter 0)))
  (if (Utilities|Array|ContainsItem (Variables|/Game/Cold_Case/Blueprints/BP_Player.BP_Player_C|GetInventory _asbp_player) "Keys")
    (Audio|PlaySoundatLocation "/Game/Cold_Case/Audio/SFX/494128__wlabarron__hotel-room-door-unlocking.494128__wlabarron__hotel-room-door-unlocking" (Transformation|GetActorLocation) "0, 0, 0" 1.0 1.0 0.0 0 0 0 0)
    (bind _returnvalue (Sequencer|Player|CreateLevelSequencePlayer (Variables|Default|GetDoorSequence)))
    (Sequencer|Player|Play _returnvalue :!class /Script/MovieScene.MovieSceneSequencePlayer)
    (EventDispatchers|AssignOnFinished _returnvalue (delegate Custom|OnFinished_Event_0))))

(fn ConstructionScript
  (|CallParentFunction))