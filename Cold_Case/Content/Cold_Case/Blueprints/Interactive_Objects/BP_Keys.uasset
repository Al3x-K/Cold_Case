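; BP_Keys is an interactive pickup that gives the player the keys, presented as their way out.
; On ExecuteInteraction it adds "Keys" to the BP_Player inventory and shows a WBP_Collectable widget with the name and flavor text.
; After a short delay it removes the widget, plays a jingling sound at its location and destroys itself.
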(event EventExecuteInteraction
  (bind _asbp_player (Utilities|Casting|CastToBP_Player (Game|GetPlayerCharacter 0)))
  (Utilities|Array|Add (Variables|/Game/Cold_Case/Blueprints/BP_Player.BP_Player_C|GetInventory _asbp_player) "Keys")
  (bind _returnvalue (UserInterface|CreateWidget "/Game/Cold_Case/UI/WBP_Collectable.WBP_Collectable_C" (Game|GetPlayerController 0)))
  (Default|UpdateText _returnvalue "Keys " "There they are. My way out.")
  (UserInterface|Viewport|AddtoViewport _returnvalue 0)
  (Utilities|FlowControl|Delay 2.5)
  (Widget|RemovefromParent _returnvalue)
  (Audio|PlaySoundatLocation "/Game/Cold_Case/Audio/SFX/750832__ozna__the-sound-of-keys-jiggling.750832__ozna__the-sound-of-keys-jiggling" (Transformation|GetActorLocation) "0, 0, 0" 1.0 1.0 0.0 0 0 0 0)
  (Actor|DestroyActor))

(fn ConstructionScript
  (|CallParentFunction))