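; BP_Recorder1 is an interactable tape recorder in Cold_Case that needs a cassette from the player's inventory.
; ExecuteInteraction snaps it to the player's InspectionAnchor, halts walking and shows a timed description, then calls AttemptPlayTape and immediately restores the recorder and movement without awaiting its delays.
; AttemptPlayTape either consumes "Casette" and briefly shows a W_FinalClue use prompt, or plays static with a "Missing tape" message.
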(event Custom|AttemptPlayTape
  (bind _asbp_player (Utilities|Casting|CastToBP_Player (Game|GetPlayerCharacter 0)))
  (if (Utilities|Array|ContainsItem (Variables|/Game/Cold_Case/Blueprints/BP_Player.BP_Player_C|GetInventory _asbp_player) "Casette")
    (Audio|PlaySound2D "/Game/Cold_Case/Audio/SFX/848795__swifty433__pickup.848795__swifty433__pickup" 1.0 1.0 0.0 0 0)
    (bind _returnvalue (UserInterface|CreateWidget "/Game/Cold_Case/UI/W_FinalClue.W_FinalClue_C" (Game|GetPlayerController 0)))
    (Variables|Default|SetFinalClueWidget _returnvalue)
    (Default|UpdateUI _returnvalue "Recorder" "Press F to use.")
    (UserInterface|Viewport|AddtoViewport _returnvalue 0)
    (Utilities|Array|RemoveItem (Variables|/Game/Cold_Case/Blueprints/BP_Player.BP_Player_C|GetInventory _asbp_player) "Casette")
    (Utilities|FlowControl|Delay 1.5)
    (Widget|RemovefromParent _returnvalue)
    (else
      (Audio|PlaySound2D "/Game/Cold_Case/Audio/SFX/818440__froey__static-cutting-out.818440__froey__static-cutting-out" 1.0 1.0 0.0 0 0)
      (bind _returnvalue_2 (UserInterface|CreateWidget "/Game/Cold_Case/UI/WBP_Collectable.WBP_Collectable_C" (Game|GetPlayerController 0)))
      (Default|UpdateText _returnvalue_2 "Recorder" "Missing tape")
      (UserInterface|Viewport|AddtoViewport _returnvalue_2 0)
      (Utilities|FlowControl|Delay 4.0)
      (Widget|RemovefromParent _returnvalue_2))))

(event EventExecuteInteraction
  (bind _asbp_player (Utilities|Casting|CastToBP_Player (Game|GetPlayerCharacter 0)))
  (Variables|Default|Setoriginaltransform (Transformation|GetActorTransform))
  (Transformation|AttachComponentToComponent (Variables|/Game/Cold_Case/Blueprints/BP_Player.BP_Player_C|GetInspectionAnchor _asbp_player) "None" "SnapToTarget" "SnapToTarget" "SnapToTarget" true)
  (Collision|SetActorEnableCollision false)
  (Transformation|SetActorRotation "20.000000,90.000000,-20.000000")
  (Variables|/Script/Engine.CharacterMovementComponent|SetMaxWalkSpeed (Variables|/Script/Engine.Character|GetCharacterMovement _asbp_player) 0.0)
  (bind _returnvalue (UserInterface|CreateWidget "/Game/Cold_Case/UI/WBP_Collectable.WBP_Collectable_C"))
  (Default|UpdateText _returnvalue "Recorder" "There it is. Been in this drawer for months. Let's see if it still works.")
  (UserInterface|Viewport|AddtoViewport _returnvalue 0)
  (Utilities|FlowControl|Delay 2.0)
  (Widget|RemovefromParent _returnvalue)
  (CallFunction|AttemptPlayTape)
  (Transformation|DetachFromActor "KeepWorld" "KeepWorld" "KeepWorld")
  (Transformation|SetActorTransform (Variables|Default|Getoriginaltransform))
  (Collision|SetActorEnableCollision true)
  (Variables|/Script/Engine.CharacterMovementComponent|SetMaxWalkSpeed (Variables|/Script/Engine.Character|GetCharacterMovement _asbp_player) 2.5e+02))

(fn ConstructionScript
  (|CallParentFunction))