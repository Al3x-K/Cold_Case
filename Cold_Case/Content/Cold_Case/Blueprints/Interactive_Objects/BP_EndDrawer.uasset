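; BP_EndDrawer is an interactive drawer that opens only once the player has used the recorder.
; Its ExecuteInteraction event casts the player character to BP_Player and checks the UsedRecorder flag.
; If set, it plays the DrawerSlide timeline to lerp the Drawer's relative location outward along Y while playing a movement sound.
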(event EventExecuteInteraction
  (bind _asbp_player (Utilities|Casting|CastToBP_Player (Game|GetPlayerCharacter 0)))
  (if (Variables|/Game/Cold_Case/Blueprints/BP_Player.BP_Player_C|GetUsedRecorder _asbp_player)
    (Utilities|FlowControl|Sequence
      (:then_0
        (bind _alpha (Timeline|DrawerSlide Play)
          (:Update
            (Transformation|SetRelativeLocation (Variables|Default|GetDrawer) (Math|Vector|Lerp(Vector) "0, 0, 0" "0.000000,40.000000,0.000000" _alpha) false false))))
      (:then_1
        (Audio|Components|Audio|Play (Variables|Default|GetMovementSound) 0.0)))))

(fn ConstructionScript)