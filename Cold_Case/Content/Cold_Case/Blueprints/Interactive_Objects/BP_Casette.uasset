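; BP_Casette is an interactive cassette pickup, a recorded backup from the Harlow case that needs a device to play it.
; On interaction it adds "Cassette" to the BP_Player inventory, hides the main HUD and shows a WBP_Collectable name and description popup.
; After a short delay it removes the popup, plays a pickup sound, destroys itself and restores the HUD.
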(event EventExecuteInteraction
  (bind _asbp_player (Utilities|Casting|CastToBP_Player (Game|GetPlayerCharacter 0)))
  (Widget|SetVisibility (Variables|/Game/Cold_Case/Blueprints/BP_Player.BP_Player_C|GetMainHUDReference _asbp_player) "Hidden")
  (Utilities|Array|Add (Variables|/Game/Cold_Case/Blueprints/BP_Player.BP_Player_C|GetInventory _asbp_player) "Cassette")
  (bind _returnvalue (UserInterface|CreateWidget "/Game/Cold_Case/UI/WBP_Collectable.WBP_Collectable_C" (Game|GetPlayerController 0)))
  (Default|UpdateText _returnvalue "Cassette" "A recorded backup from the Harlow case. I need something to play this on.")
  (UserInterface|Viewport|AddtoViewport _returnvalue 0)
  (Utilities|FlowControl|Delay 2.0)
  (Widget|RemovefromParent _returnvalue)
  (Audio|PlaySoundatLocation "/Game/Cold_Case/Audio/SFX/848795__swifty433__pickup.848795__swifty433__pickup" (Transformation|GetActorLocation) "0, 0, 0" 1.0 1.0 0.0 0 0 0 0)
  (Actor|DestroyActor)
  (Widget|SetVisibility (Variables|/Game/Cold_Case/Blueprints/BP_Player.BP_Player_C|GetMainHUDReference _asbp_player) "Visible"))

(fn ConstructionScript
  (|CallParentFunction))